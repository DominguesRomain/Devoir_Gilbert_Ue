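; BP_Door_1 is a door that swings instantly between closed and open by snapping Cube1's relative yaw between 0 and 90 degrees.
; Activate and Desactivate both call the same toggle, which also runs at BeginPlay when Open is set.
; Each toggle raises or lowers the OpenDoors count on a referenced Lamp and calls its LightDoor to update it.
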(event `self.ReceiveBeginPlay`
  (if (`self.Open?`)
    (`self.Toggle Door`)))

(event `/Game/Blueprint/void/BPI_NewInterrupteur.Activate`
  (`self.Toggle Door`))

(event `/Game/Blueprint/void/BPI_NewInterrupteur.Desactivate`
  (`self.Toggle Door`))

(fn `LightOff`
  (bind _lamp (`self.lamp`))
  (`/Engine/EditorBlueprintResources/StandardMacros.DecrementInt` (`/Game/Blueprint/Light/BP_Light_1.OpenDoors` _lamp)
    (:`  `
      (`/Game/Blueprint/Light/BP_Light_1.Light Door` _lamp))))

(fn `LightOn`
  (bind _lamp (`self.lamp`))
  (`/Engine/EditorBlueprintResources/StandardMacros.IncrementInt` (`/Game/Blueprint/Light/BP_Light_1.OpenDoors` _lamp)
    (:`  `
      (`/Game/Blueprint/Light/BP_Light_1.Light Door` _lamp))))

(fn `Toggle Door`
  (bind _cube1 (`self.Cube1`))
  (bind (_relativerotation_roll _relativerotation_pitch _relativerotation_yaw) (`KismetMathLibrary.BreakRotator` (`SceneComponent.RelativeRotation` _cube1)))
  (if (== _relativerotation_yaw 90.0)
    (`SceneComponent.K2_SetRelativeRotation` :`self` _cube1)
    (`self.LightOff`)
    (else
      (`SceneComponent.K2_SetRelativeRotation` _cube1 (struct :`Yaw` 90.0) false false)
      (`self.LightOn`))))

(fn `UserConstructionScript`)