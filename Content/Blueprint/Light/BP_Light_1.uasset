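; BP_Light_1 is a light Blueprint with a point light that can be toggled or driven by a count of open doors.
; ToggleLight flips the light's visibility.
; Light Door prints the OpenDoors value, then shows the light when it is below one and hides it otherwise.
; The file contains no logic that changes OpenDoors or calls either function.
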(fn `Light Door`
  (bind _opendoors (`self.OpenDoors`))
  (bind _pointlight (`self.PointLight`))
  (`KismetSystemLibrary.PrintString` (`KismetStringLibrary.Conv_IntToString` _opendoors))
  (if (< _opendoors 1)
    (`SceneComponent.SetVisibility` _pointlight true false)
    (else
      (`SceneComponent.SetVisibility` _pointlight false false))))

(fn `ToggleLight`
  (bind _pointlight (`self.PointLight`))
  (`SceneComponent.SetVisibility` _pointlight (not (`SceneComponent.bVisible` _pointlight)) false))

(fn `UserConstructionScript`)